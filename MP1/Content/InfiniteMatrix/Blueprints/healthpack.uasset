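; Health pack pickup actor that heals the player on contact and penalizes shooting it.
; A box overlap from BP_Player adds a fixed amount of health, or sets it to the cap if already at or above it, and consumes the pack either way.
; An overlap from bp_projectile instead deducts score from the first player's pawn and destroys the pack.
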(event OnComponentBeginOverlap(Box)
  (params (OverlappedComponent :type Primitive%20Component%20Object%20Reference) (OtherActor :type Actor%20Object%20Reference) (OtherComp :type Primitive%20Component%20Object%20Reference) (OtherBodyIndex :type Integer) (bFromSweep :type Boolean) (SweepResult :type Hit%20Result%20Structure%20%28by%20ref%29))
  (Utilities|Casting|CastTobp_projectile OtherActor
    (:then
      (bind _asbp_player (Utilities|Casting|CastToBP_Player (Game|Player|GetPlayerPawn 0)))
      (Variables|/Game/InfiniteMatrix/Blueprints/BP_Player.BP_Player_C|Setscore _asbp_player (- (Variables|/Game/InfiniteMatrix/Blueprints/BP_Player.BP_Player_C|Getscore _asbp_player) 30))
      (Actor|DestroyActor))
    (:CastFailed
      (bind _asbp_player_2 (Utilities|Casting|CastToBP_Player OtherActor))
      (if (>= (Variables|/Game/InfiniteMatrix/Blueprints/BP_Player.BP_Player_C|Gethealth _asbp_player_2) 1e+02)
        (Variables|/Game/InfiniteMatrix/Blueprints/BP_Player.BP_Player_C|Sethealth _asbp_player_2 1e+02)
        (Actor|DestroyActor)
        (else
          (Variables|/Game/InfiniteMatrix/Blueprints/BP_Player.BP_Player_C|Sethealth _asbp_player_2 (+ (Variables|/Game/InfiniteMatrix/Blueprints/BP_Player.BP_Player_C|Gethealth _asbp_player_2) 1e+01))
          (Actor|DestroyActor))))))

(event EventBeginPlay)

(event Collision|EventActorBeginOverlap
  (params (OtherActor :type Actor%20Object%20Reference)))

(event EventTick
  (params (DeltaSeconds :type Float%20%28single-precision%29)))

(fn ConstructionScript)